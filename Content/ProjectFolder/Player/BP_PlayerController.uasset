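; BP_PlayerController is a player controller that handles the whistle and interact inputs.
; Whistling, blocked while hiding, plays a sound at the player character and reports a tagged noise event for AI hearing, then locks behind a short timer-based cooldown.
; Interact forwards the triggered, started and canceled input phases to the current interactable, passing the controller along.
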(event Custom|ResetWhistleAction
  (Variables|Default|SetIsWhistleAvailable true))

(event Input|EnhancedActionEvents|EnhancedInputActionIA_Whistle
  (params (ActionValue :type Boolean) (ElapsedSeconds :type Float%20%28double-precision%29) (TriggeredSeconds :type Float%20%28double-precision%29) (InputAction :type Input%20Action%20Object%20Reference :default "/Game/ProjectFolder/Input/Actions/IA_Whistle.IA_Whistle"))
  (bind _returnvalue (Game|GetPlayerCharacter 0))
  (bind _returnvalue_2 (Transformation|GetActorLocation _returnvalue))
  (if (and (Variables|Default|GetIsWhistleAvailable) (not (Class|ProjectAIDirectorPlayerController|GetIsHiding)))
    (Audio|PlaySoundatLocation "/Game/ProjectFolder/Audio/male-whistle.male-whistle" _returnvalue_2 "0, 0, 0" 1.0 1.0 0.0 0 0 0 0)
    (Class|AISenseHearing|ReportNoiseEvent _returnvalue_2 1.0 _returnvalue 0.0 "Whistle")
    (Variables|Default|SetIsWhistleAvailable false)
    (Utilities|Time|SetTimerbyEvent (delegate Custom|ResetWhistleAction) 1.0)))

(event Input|EnhancedActionEvents|EnhancedInputActionIA_Interact
  (params (ActionValue :type Boolean) (ElapsedSeconds :type Float%20%28double-precision%29) (TriggeredSeconds :type Float%20%28double-precision%29) (InputAction :type Input%20Action%20Object%20Reference :default "/Game/ProjectFolder/Input/Actions/IA_Interact.IA_Interact"))
  (bind _currentinteractable (Variables|Default|GetCurrentInteractable))
  (bind _currentinteractable_2 (Variables|Default|GetCurrentInteractable))
  (bind _currentinteractable_3 (Variables|Default|GetCurrentInteractable))
  (:Triggered
    (if (Utilities|IsValid _currentinteractable_2)
      (Default|TriggerInteraction _currentinteractable_2 self)))
  (:Started
    (if (Utilities|IsValid _currentinteractable_3)
      (Default|StartInteraction _currentinteractable_3 self)))
  (:Canceled
    (if (Utilities|IsValid _currentinteractable)
      (Default|CancelInteraction _currentinteractable self))))

(fn ConstructionScript)