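; BP_PlayerCharacter is the player character, which reports nearby interactable actors to its player controller.
; Overlapping an actor tagged Interactable stores it as CurrentInteractable on BP_PlayerController if it casts to BP_Interactable.
; Ending the overlap clears that reference only if it is still the current one and the player is not hiding.
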(event Collision|EventActorBeginOverlap
  (params (OtherActor :type Actor%20Object%20Reference))
  (if (Actor|ActorHasTag OtherActor "Interactable")
    (bind _asbp_player_controller (Utilities|Casting|CastToBP_PlayerController (Pawn|GetController)))
    (bind _asbp_interactable (Utilities|Casting|CastToBP_Interactable OtherActor))
    (Variables|/Game/ProjectFolder/Player/BP_PlayerController.BP_PlayerController_C|SetCurrentInteractable _asbp_player_controller _asbp_interactable)))

(event Collision|EventActorEndOverlap
  (params (OtherActor :type Actor%20Object%20Reference))
  (if (Actor|ActorHasTag OtherActor "Interactable")
    (bind _asbp_player_controller (Utilities|Casting|CastToBP_PlayerController (Pawn|GetController)))
    (if (not (Class|ProjectAIDirectorPlayerController|GetIsHiding _asbp_player_controller))
      (bind _asbp_interactable (Utilities|Casting|CastToBP_Interactable OtherActor))
      (if (== _asbp_interactable (Variables|/Game/ProjectFolder/Player/BP_PlayerController.BP_PlayerController_C|GetCurrentInteractable _asbp_player_controller))
        (Variables|/Game/ProjectFolder/Player/BP_PlayerController.BP_PlayerController_C|SetCurrentInteractable _asbp_player_controller 0)))))

(fn ConstructionScript)