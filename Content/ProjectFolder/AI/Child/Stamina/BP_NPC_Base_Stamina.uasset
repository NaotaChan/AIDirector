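; Base NPC Blueprint that adds a stamina system, shown through a stamina widget bar, to its parent AI character.
; Tick runs a looping timer while the NPC moves, draining stamina at a walk or run rate based on its speed type, and clears it when idle.
; Low stamina switches the NPC from running to walking; empty stamina ragdolls the mesh, stops the AI brain and hides the bar.
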(event Custom|ReduceStamina
  (bind _staminadecay_walk (Variables|Default|GetStaminaDecay_Walk))
  (bind _output_get (Variables|Default|SetCurrentStamina (- (Variables|Default|GetCurrentStamina) (Utilities|Select :Index (Class|AIBaseNPC|GetCurrentSpeedType) :UNSET _staminadecay_walk :WALK _staminadecay_walk :RUN (Variables|Default|GetStaminaDecay_Run)))))
  (bind _output_get_2 (Variables|/Game/ProjectFolder/UI/UW_StaminaBar.UW_StaminaBar_C|SetCurrentStamina (Variables|Default|GetStaminaWidgetRef) _output_get))
  (if (<= _output_get_2 0.0)
    (Collision|SetCollisionProfileName (Variables|Character|GetMesh) "Ragdoll" true :!class /Script/Engine.PrimitiveComponent)
    (Physics|SetSimulatePhysics (Variables|Character|GetMesh) true)
    (AI|Logic|StopLogic (Variables|/Script/AIModule.AIController|GetBrainComponent (Class|AIBaseNPC|GetAICRef)) "Dead")
    (Utilities|Time|ClearandInvalidateTimerbyHandle (Variables|Default|GetStaminaDecayTimeHandler))
    (Widget|SetVisibility (Variables|Default|GetStaminaWidgetRef) "Hidden")
    (elif (<= _output_get_2 3e+01)
      (Class|AIBaseNPC|ChangeSpeedType "WALK"))))

(event EventBeginPlay
  (|CallParentFunction)
  (Variables|Default|SetCurrentStamina (Variables|Default|GetMaxStamina))
  (bind _asuw_stamina_bar (Utilities|Casting|CastToUW_StaminaBar (UserInterface|GetUserWidgetObject (Variables|Default|GetStaminaWidget))))
  (bind _output_get (Variables|Default|SetStaminaWidgetRef _asuw_stamina_bar))
  (Variables|/Game/ProjectFolder/UI/UW_StaminaBar.UW_StaminaBar_C|SetMaxStamina _output_get (Variables|Default|GetMaxStamina))
  (Variables|/Game/ProjectFolder/UI/UW_StaminaBar.UW_StaminaBar_C|SetCurrentStamina (Variables|Default|GetStaminaWidgetRef) (Variables|Default|GetCurrentStamina))
  (Class|AIBaseNPC|ChangeSpeedType "RUN"))

(event EventTick
  (params (DeltaSeconds :type Float%20%28single-precision%29))
  (|CallParentFunction DeltaSeconds)
  (bind _output_get (Variables|Default|SetIsMoving (> (Math|Vector|VectorLengthXY (Variables|/Script/Engine.MovementComponent|GetVelocity (Variables|Character|GetCharacterMovement))) 3.0)))
  (if _output_get
    (if (not (Utilities|Time|IsValidTimerHandle (Variables|Default|GetStaminaDecayTimeHandler)))
      (bind _returnvalue (Utilities|Time|SetTimerbyEvent (delegate Custom|ReduceStamina) (Variables|Default|GetStaminaDecayTimer) true))
      (Variables|Default|SetStaminaDecayTimeHandler _returnvalue))
    (else
      (Utilities|Time|ClearandInvalidateTimerbyHandle (Variables|Default|GetStaminaDecayTimeHandler)))))

(fn ConstructionScript
  (|CallParentFunction))