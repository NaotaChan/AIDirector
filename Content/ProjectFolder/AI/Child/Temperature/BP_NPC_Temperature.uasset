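; NPC child Blueprint that adds a body temperature survival mechanic, shown on a widget bar.
; A looping timer drains temperature at a rate set by whether the NPC is moving and its speed type.
; StartHeatingUp swaps the drain for a looping heat timer until StopHeatingUp restores it.
; Reaching either the cold or hot limit triggers Death, which ragdolls the mesh, stops AI logic and hides the bar.
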(event Custom|ReduceTemperature
  (bind _output_get (Variables|Default|SetCurrentTemperature (- (Variables|Default|GetCurrentTemperature) (Math|Float|SelectFloat (Utilities|Select :Index (Class|AIBaseNPC|GetCurrentSpeedType) :UNSET 0.0 :WALK 1.0 :RUN (Variables|Default|GetTemperatureDecay_Movement)) (Variables|Default|GetTemperatureDecay_Still) (Variables|Default|GetIsMoving)))))
  (bind _output_get_2 (Variables|/Game/ProjectFolder/UI/UW_TemperatureBar.UW_TemperatureBar_C|SetCurrentTemperature (Variables|Default|GetTemperatureBarWidget) _output_get))
  (if (<= _output_get_2 0.0)
    (CallFunction|Death)))

(event Custom|StartHeatingUp
  (params (HeatStrenght :type Float%20%28double-precision%29))
  (if (not (Utilities|Time|IsValidTimerHandle (Variables|Default|GetHeatingTimeHandler)))
    (Variables|Default|SetHeatValue HeatStrenght)
    (bind _returnvalue (Utilities|Time|SetTimerbyEvent (EventDispatchers|CreateEvent :!event Custom|HeatingUp) (Variables|Default|GetHeatingTimer) true))
    (Variables|Default|SetHeatingTimeHandler _returnvalue)
    (CallFunction|StopReduceTemperature)))

(event Custom|HeatingUp
  (bind _output_get (Variables|Default|SetCurrentTemperature (Math|Float|Clamp(Float) (+ (Variables|Default|GetCurrentTemperature) (Variables|Default|GetHeatValue)) 0.0 1e+02)))
  (bind _output_get_2 (Variables|/Game/ProjectFolder/UI/UW_TemperatureBar.UW_TemperatureBar_C|SetCurrentTemperature (Variables|Default|GetTemperatureBarWidget) _output_get))
  (if (>= _output_get_2 1e+02)
    (CallFunction|Death)))

(event Custom|StopHeatingUp
  (Utilities|Time|ClearandInvalidateTimerbyHandle (Variables|Default|GetHeatingTimeHandler))
  (CallFunction|StartReduceTemperature))

(event Custom|StartReduceTemperature
  (bind _returnvalue (Utilities|Time|SetTimerbyEvent (EventDispatchers|CreateEvent :!event Custom|ReduceTemperature) (Variables|Default|GetTemperatureDecayTimer) true))
  (Variables|Default|SetTemperatureDecayTimeHandler _returnvalue))

(event Custom|StopReduceTemperature
  (Utilities|Time|ClearandInvalidateTimerbyHandle (Variables|Default|GetTemperatureDecayTimeHandler)))

(event Custom|Death
  (Collision|SetCollisionProfileName (Variables|Character|GetMesh) "Ragdoll" true :!class /Script/Engine.PrimitiveComponent)
  (Physics|SetSimulatePhysics (Variables|Character|GetMesh) true)
  (AI|Logic|StopLogic (Variables|/Script/AIModule.AIController|GetBrainComponent (Class|AIBaseNPC|GetAICRef)) "Dead")
  (Utilities|Time|ClearandInvalidateTimerbyHandle (Variables|Default|GetTemperatureDecayTimeHandler))
  (Rendering|SetVisibility (Variables|Default|GetTemperatureWidget) false false))

(event EventBeginPlay
  (|CallParentFunction)
  (Variables|Default|SetCurrentTemperature 45.0)
  (bind _asuw_temperature_bar (Utilities|Casting|CastToUW_TemperatureBar (UserInterface|GetUserWidgetObject (Variables|Default|GetTemperatureWidget))))
  (bind _output_get (Variables|Default|SetTemperatureBarWidget _asuw_temperature_bar))
  (Variables|/Game/ProjectFolder/UI/UW_TemperatureBar.UW_TemperatureBar_C|SetMaxTemperature _output_get (Variables|Default|GetMaxTemperature))
  (Variables|/Game/ProjectFolder/UI/UW_TemperatureBar.UW_TemperatureBar_C|SetCurrentTemperature (Variables|Default|GetTemperatureBarWidget) (Variables|Default|GetCurrentTemperature))
  (CallFunction|StartReduceTemperature))

(event EventTick
  (params (DeltaSeconds :type Float%20%28single-precision%29))
  (|CallParentFunction DeltaSeconds)
  (Variables|Default|SetIsMoving (> (Math|Vector|VectorLengthXY (Variables|/Script/Engine.MovementComponent|GetVelocity (Variables|Character|GetCharacterMovement))) 3.0)))

(fn ConstructionScript
  (|CallParentFunction))

(fn GetCurrentTemperatureValue
  (return (Variables|Default|GetCurrentTemperature)))