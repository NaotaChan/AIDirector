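; AI controller for temperature NPCs that reacts to both sight and a heat sense.
; On possess it caches the controlled BP_NPC_Temperature, then routes perception updates by sense class.
; Sight sets the blackboard Target, or clears it and the suspicion key when lost.
; Heat tells the NPC to start heating up at the stimulus strength, or to stop when the stimulus ends.
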(event EventActorPerceivedUpdate
  (params (UpdatedActor :type Actor%20Object%20Reference) (Stimulus :type AI%20Stimulus%20Structure))
  (bind (_strength _bsuccessfullysensed) (Utilities|Struct|BreakAIStimulus Stimulus))
  (bind _returnvalue (Class|AIPerceptionSystem|GetSenseClassforStimulus Stimulus))
  (if (== _returnvalue "/Script/AIModule.AISense_Sight")
    (if _bsuccessfullysensed
      (AI|Components|Blackboard|SetValueasObject (Variables|Default|GetBlackboard) (Utilities|Name|MakeLiteralName "Target") UpdatedActor)
      (else
        (AI|Components|Blackboard|ClearValue (Variables|Default|GetBlackboard) (Utilities|Name|MakeLiteralName "Target"))
        (AI|Components|Blackboard|ClearValue (Variables|Default|GetBlackboard) (Utilities|Name|MakeLiteralName "IsSupsicious"))))
    (elif (== _returnvalue "/Script/Project_AIDirector.AISense_Heat")
      (if _bsuccessfullysensed
        (Default|StartHeatingUp (Variables|Default|GetTemperatureNPCRef) _strength)
        (else
          (Default|StopHeatingUp (Variables|Default|GetTemperatureNPCRef)))))))

(event EventPossess
  (params (PossessedPawn :type Pawn%20Object%20Reference))
  (|CallParentFunction PossessedPawn)
  (bind _asbp_npc_temperature (Utilities|Casting|CastToBP_NPC_Temperature (Class|AIBaseController|GetNPCRef)))
  (Variables|Default|SetTemperatureNPCRef _asbp_npc_temperature))

(fn ConstructionScript
  (|CallParentFunction))