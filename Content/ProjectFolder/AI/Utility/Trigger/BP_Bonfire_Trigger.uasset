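; Bonfire rest-area trigger that tells temperature-aware NPCs when they start or stop heating up.
; Box overlap begin and end store the BP_NPC_Temperature actor and send a heat event with the trigger's location, strength and a heating flag.
; The construction script sizes the box from an editable extent and scales an optional debug mesh to match.
; Looping-timer logic for repeated reports is present but unconnected.
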(event OnComponentBeginOverlap(RestAreaColliderTrigger)
  (params (OverlappedComponent :type Primitive%20Component%20Object%20Reference) (OtherActor :type Actor%20Object%20Reference) (OtherComp :type Primitive%20Component%20Object%20Reference) (OtherBodyIndex :type Integer) (bFromSweep :type Boolean) (SweepResult :type Hit%20Result%20Structure%20%28by%20ref%29))
  (bind _asbp_npc_temperature (Utilities|Casting|CastToBP_NPC_Temperature OtherActor))
  (Variables|Default|SetNPCRef _asbp_npc_temperature)
  (CallFunction|ReportHeat true))

(event OnComponentEndOverlap(RestAreaColliderTrigger)
  (params (OverlappedComponent :type Primitive%20Component%20Object%20Reference) (OtherActor :type Actor%20Object%20Reference) (OtherComp :type Primitive%20Component%20Object%20Reference) (OtherBodyIndex :type Integer))
  (bind _asbp_npc_temperature (Utilities|Casting|CastToBP_NPC_Temperature OtherActor))
  (Variables|Default|SetNPCRef _asbp_npc_temperature)
  (CallFunction|ReportHeat false))

(event Custom|ReportHeat
  (params (IsSuccessfullyHeatingUp :type Boolean))
  (Class|AISenseHeat|ReportHeatEvent self (Variables|Default|GetNPCRef) (Transformation|GetActorLocation) (Variables|Default|GetStrenght) IsSuccessfullyHeatingUp))

(event EventBeginPlay)

(event Collision|EventActorBeginOverlap
  (params (OtherActor :type Actor%20Object%20Reference)))

(event EventTick
  (params (DeltaSeconds :type Float%20%28single-precision%29)))

(fn ConstructionScript
  (Components|Box|SetBoxExtent (Variables|Default|GetRestAreaColliderTrigger) (Variables|Default|GetAreaExtent) true)
  (Variables|Default|GetDebugMesh
    (:then
      (Transformation|SetRelativeScale3D (Variables|Default|GetDebugMesh) (/ (* (Variables|/Script/Engine.BoxComponent|GetBoxExtent (Variables|Default|GetRestAreaColliderTrigger)) 2.0) 1e+02))
      (Development|SetHiddeninGame (Variables|Default|GetDebugMesh) (not (Variables|Default|GetShowDebug)) false))
    (:else)))