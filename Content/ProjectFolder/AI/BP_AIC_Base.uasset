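; BP_AIC_Base is a base AI controller that runs its assigned behavior tree on BeginPlay and feeds perception results into the Blackboard.
; Sight updates set the perceived actor as Target, or clear it when sensing fails.
; A separate perception component handler reacts to stimuli tagged "Run", treated as noise, by storing the location as NoiseLocation and setting IsSuspicious.
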(event OnTargetPerceptionUpdated(PerceptionComponent)
  (params (Actor :type Actor%20Object%20Reference) (Stimulus :type AI%20Stimulus%20Structure))
  (bind (_age _expirationage _strength _stimuluslocation _receiverlocation _tag) (Utilities|Struct|BreakAIStimulus Stimulus))
  ;[0.15 0.15 0.15 0.5] Run Noise
  (if (== _tag "Run")
    (AI|Components|Blackboard|SetValueasVector (AI|GetBlackboard 0) (Utilities|Name|MakeLiteralName "NoiseLocation") _stimuluslocation)
    (AI|Components|Blackboard|SetValueasBool (AI|GetBlackboard 0) (Utilities|Name|MakeLiteralName "IsSuspicious") true)))

(event EventBeginPlay
  (AI|RunBehaviorTree (Variables|Default|GetBTAsset)))

(event EventActorPerceivedUpdate
  (params (UpdatedActor :type Actor%20Object%20Reference) (Stimulus :type AI%20Stimulus%20Structure))
  (bind _returnvalue (Class|AIPerceptionSystem|GetSenseClassforStimulus Stimulus))
  (if (== _returnvalue "/Script/AIModule.AISense_Sight")
    (if (.bSuccessfullySensed (Utilities|Struct|BreakAIStimulus Stimulus))
      (AI|Components|Blackboard|SetValueasObject (Variables|Default|GetBlackboard) (Utilities|Name|MakeLiteralName "Target") UpdatedActor)
      (else
        (AI|Components|Blackboard|ClearValue (Variables|Default|GetBlackboard) (Utilities|Name|MakeLiteralName "Target"))))))

(fn ConstructionScript)