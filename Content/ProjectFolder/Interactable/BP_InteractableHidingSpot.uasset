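; Interactable hiding spot that shows a prompt when the player overlaps it and toggles the player controller's hiding state when interaction triggers.
; Starting an interaction disables movement and runs a timeline-driven fill bar; cancelling restores walking unless already hidden.
; Hiding saves the capsule position, slides the mesh toward the spot, teleports the capsule there and disables its collision.
; Unhiding restores position, mesh, collision and walking.
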(event EventBeginPlay
  (|CallParentFunction)
  (Rendering|SetVisibility (Variables|Default|GetStartHidingWidget) false false)
  (Rendering|SetVisibility (Variables|Default|GetStopHidingWidget) false false)
  (Rendering|SetVisibility (Variables|Default|GetFillBarWidget) false false))

(event Collision|EventActorBeginOverlap
  (params (OtherActor :type Actor%20Object%20Reference))
  (|CallParentFunction OtherActor)
  (if (Actor|ActorHasTag OtherActor "Player")
    (Rendering|SetVisibility (Variables|Default|GetStartHidingWidget) true false)))

(event EventTriggerInteraction
  (params (Interactor :type Actor%20Object%20Reference))
  (bind _returnvalue (Game|GetPlayerCharacter 0))
  (bind _returnvalue_2 (Game|GetPlayerCharacter 0))
  (bind _interactioncollision (Variables|Default|GetInteractionCollision))
  (bind _returnvalue_3 (Transformation|GetWorldLocation _interactioncollision))
  (bind _mesh (Variables|/Script/Engine.Character|GetMesh _returnvalue_2))
  (bind _mesh_2 (Variables|/Script/Engine.Character|GetMesh _returnvalue))
  (bind _asproject_aidirector_player_controller (Utilities|Casting|CastToProject_AIDirectorPlayerController Interactor))
  (if (Class|ProjectAIDirectorPlayerController|GetIsHiding _asproject_aidirector_player_controller)
    (Class|ProjectAIDirectorPlayerController|SetIsHiding _asproject_aidirector_player_controller false)
    (Transformation|SetWorldLocation (Variables|/Script/Engine.Character|GetCapsuleComponent (Game|GetPlayerCharacter 0)) (Variables|Default|GetCurrentPlayerPosition) false true)
    (Components|MoveComponentTo _mesh_2 "0.000000,0.000000,-90.000000" (Variables|/Script/Engine.SceneComponent|GetRelativeRotation _mesh_2) false false 0.25 false)
    (Collision|SetCollisionEnabled (Variables|/Script/Engine.Character|GetCapsuleComponent (Game|GetPlayerCharacter 0)) "QueryAndPhysics")
    (Pawn|Components|CharacterMovement|SetMovementMode (Variables|/Script/Engine.Character|GetCharacterMovement (Game|GetPlayerCharacter 0)) "MOVE_Walking" 0)
    (Rendering|SetVisibility (Variables|Default|GetStartHidingWidget) true false)
    (Rendering|SetVisibility (Variables|Default|GetStopHidingWidget) false false)
    (Rendering|SetVisibility (Variables|Default|GetFillBarWidget) false false)
    (else
      (Class|ProjectAIDirectorPlayerController|SetIsHiding _asproject_aidirector_player_controller true)
      (Components|MoveComponentTo _mesh (Math|Transform|InverseTransformLocation (Transformation|GetActorTransform _returnvalue_2) (Transformation|GetActorLocation self)) (Variables|/Script/Engine.SceneComponent|GetRelativeRotation _mesh) false false 0.25 false)
      (Variables|Default|SetCurrentPlayerPosition (Transformation|GetWorldLocation (Variables|/Script/Engine.Character|GetCapsuleComponent (Game|GetPlayerCharacter 0))))
      (Transformation|SetWorldLocation (Variables|/Script/Engine.Character|GetCapsuleComponent (Game|GetPlayerCharacter 0)) (Math|Vector|MakeVector (.x _returnvalue_3) (.y _returnvalue_3) 0.0) false true)
      (Collision|SetCollisionEnabled (Variables|/Script/Engine.Character|GetCapsuleComponent (Game|GetPlayerCharacter 0)) "NoCollision")
      (Rendering|SetVisibility (Variables|Default|GetStartHidingWidget) false false)
      (Rendering|SetVisibility (Variables|Default|GetStopHidingWidget) true false)
      (Rendering|SetVisibility (Variables|Default|GetFillBarWidget) false false))))

(event EventStartInteraction
  (params (Interactor :type Actor%20Object%20Reference))
  (Pawn|Components|CharacterMovement|DisableMovement (Variables|/Script/Engine.Character|GetCharacterMovement (Game|GetPlayerCharacter 0)))
  (Development|PrintString "Interaction Started")
  (bind _aswb_fill_bar_widget (Utilities|Casting|CastToUW_FillBarWidget (UserInterface|GetWidget (Variables|Default|GetFillBarWidget))))
  (Default|ResetFillBar _aswb_fill_bar_widget)
  (Rendering|SetVisibility (Variables|Default|GetFillBarWidget) true false)
  (bind _newtrack_0 (Timeline|Timeline PlayFromStart)
    (:Update
      (Default|FillBartoPercent _aswb_fill_bar_widget _newtrack_0))))

(event EventCancelInteraction
  (params (Interactor :type Actor%20Object%20Reference))
  (bind _asproject_aidirector_player_controller (Utilities|Casting|CastToProject_AIDirectorPlayerController Interactor))
  (Rendering|SetVisibility (Variables|Default|GetFillBarWidget) false false)
  (if (not (Class|ProjectAIDirectorPlayerController|GetIsHiding _asproject_aidirector_player_controller))
    (Pawn|Components|CharacterMovement|SetMovementMode (Variables|/Script/Engine.Character|GetCharacterMovement (Game|GetPlayerCharacter 0)) "MOVE_Walking" 0)))

(event Collision|EventActorEndOverlap
  (params (OtherActor :type Actor%20Object%20Reference))
  (|CallParentFunction OtherActor)
  (if (Actor|ActorHasTag OtherActor "Player")
    (Rendering|SetVisibility (Variables|Default|GetStartHidingWidget) false false)))

(fn ConstructionScript
  (|CallParentFunction))