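; Interactable end-of-level object that wins the game when its interaction triggers.
; Player overlap with the interaction collision toggles a prompt widget.
; Starting an interaction disables movement and drives a fill-bar widget through a Timeline; cancelling hides the bar and restores walking.
; Triggering disables input, shows the game-won widget and pauses the game; the Timeline does not call the trigger itself.
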(event OnComponentBeginOverlap(InteractionCollision)
  (params (OverlappedComponent :type Primitive%20Component%20Object%20Reference) (OtherActor :type Actor%20Object%20Reference) (OtherComp :type Primitive%20Component%20Object%20Reference) (OtherBodyIndex :type Integer) (bFromSweep :type Boolean) (SweepResult :type Hit%20Result%20Structure%20%28by%20ref%29))
  (if (Actor|ActorHasTag OtherActor "Player")
    (Rendering|SetVisibility (Variables|Default|GetStartEndWidget) true false)))

(event OnComponentEndOverlap(InteractionCollision)
  (params (OverlappedComponent :type Primitive%20Component%20Object%20Reference) (OtherActor :type Actor%20Object%20Reference) (OtherComp :type Primitive%20Component%20Object%20Reference) (OtherBodyIndex :type Integer))
  (if (Actor|ActorHasTag OtherActor "Player")
    (Rendering|SetVisibility (Variables|Default|GetStartEndWidget) false false)))

(event EventBeginPlay
  (|CallParentFunction)
  (Rendering|SetVisibility (Variables|Default|GetStartEndWidget) false false)
  (Rendering|SetVisibility (Variables|Default|GetFillBarWidget) false false))

(event EventTriggerInteraction
  (params (Interactor :type Actor%20Object%20Reference))
  (Input|DisableInput (Game|GetPlayerCharacter 0) (Game|GetPlayerController 0))
  (Variables|/Script/Engine.CharacterMovementComponent|SetMaxWalkSpeed (Variables|/Script/Engine.Character|GetCharacterMovement (Game|GetPlayerCharacter 0)) 0.0)
  (bind _returnvalue (UserInterface|CreateWidget "/Game/ProjectFolder/UI/UW_GameWon.UW_GameWon_C" (Game|GetPlayerController 0)))
  (UserInterface|Viewport|AddtoViewport _returnvalue 0)
  (Game|SetGamePaused true))

(event EventStartInteraction
  (params (Interactor :type Actor%20Object%20Reference))
  (Pawn|Components|CharacterMovement|DisableMovement (Variables|/Script/Engine.Character|GetCharacterMovement (Game|GetPlayerCharacter 0)))
  (Development|PrintString "Interaction Started")
  (bind _aswb_fill_bar_widget (Utilities|Casting|CastToUW_FillBarWidget (UserInterface|GetWidget (Variables|Default|GetFillBarWidget))))
  (Default|ResetFillBar _aswb_fill_bar_widget)
  (Rendering|SetVisibility (Variables|Default|GetFillBarWidget) true false)
  (bind _percentage (Timeline|Timeline PlayFromStart)
    (:Update
      (Default|FillBartoPercent _aswb_fill_bar_widget _percentage))))

(event EventCancelInteraction
  (params (Interactor :type Actor%20Object%20Reference))
  (Utilities|Casting|CastToProject_AIDirectorPlayerController Interactor)
  (Rendering|SetVisibility (Variables|Default|GetFillBarWidget) false false)
  (Pawn|Components|CharacterMovement|SetMovementMode (Variables|/Script/Engine.Character|GetCharacterMovement (Game|GetPlayerCharacter 0)) "MOVE_Walking" 0))

(fn ConstructionScript
  (|CallParentFunction))